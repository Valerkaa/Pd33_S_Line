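; BP_Checkpoint is a racing checkpoint that registers vehicles crossing its trigger box.
; On overlap by a WheeledVehiclePawn, it counts the crossing up to MaxUsage, fires its crossed dispatchers, one carrying TimeToAdd, and plays a 2D sound.
; Listeners handle the outcome; a direct call to GM_RacingGame's finish-line function is left unconnected and never runs.
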(event OnComponentBeginOverlap(TriggerBox)
  (params (OverlappedComponent :type Primitive%20Component%20Object%20Reference) (OtherActor :type Actor%20Object%20Reference) (OtherComp :type Primitive%20Component%20Object%20Reference) (OtherBodyIndex :type Integer) (bFromSweep :type Boolean) (SweepResult :type Hit%20Result%20Structure%20%28by%20ref%29))
  (Utilities|Casting|CastToWheeledVehiclePawn OtherActor)
  (if (< (Variables|Default|GetCrossCounts) (Variables|Default|GetMaxUsage))
    (Math|Integer|IncrementInt (Variables|Default|GetCrossCounts)
      (:%20%20
        (Default|CallOnCheckpointCrossed)
        (Default|CallOnCheckpointCrossedwithTime (Variables|Default|GetTimeToAdd))
        (Audio|PlaySound2D "/Game/MyGame/SoundAsset/SFX_CheckpointCrossed.SFX_CheckpointCrossed" 1.0 1.0 0.0 0 0)))))

(event EventBeginPlay)

(event Collision|EventActorBeginOverlap
  (params (OtherActor :type Actor%20Object%20Reference)))

(event EventTick
  (params (DeltaSeconds :type Float%20%28single-precision%29)))

(fn ConstructionScript)