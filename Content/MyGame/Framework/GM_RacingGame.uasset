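; Game mode for a timed checkpoint race, won at the finish line and lost when time runs out.
; On BeginPlay it binds to every BP_Checkpoint, separating the finish line from checkpoints that add time.
; GameStart, not called here, starts the countdown; AddTimeToTimer re-arms it with extra time and animates the HUD.
; Either outcome shows its widget, disables input, handbrakes the car and plays level sequences tagged Win or Lose.
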(event Custom|Game%20Finish
  (params (Win :type Boolean))
  (bind _returnvalue (Game|Player|GetPlayerPawn 0))
  (Utilities|FlowControl|Sequence
    (:then_0
      (Input|DisableInput _returnvalue (Game|GetPlayerController 0))
      (bind _aswheeled_vehicle_pawn (Utilities|Casting|CastToWheeledVehiclePawn _returnvalue))
      (Class|ChaosVehicleMovementComponent|SetThrottleInput (Variables|/Script/ChaosVehicles.WheeledVehiclePawn|GetVehicleMovementComponent _aswheeled_vehicle_pawn) 0.0)
      (Class|ChaosVehicleMovementComponent|SetHandbrakeInput (Variables|/Script/ChaosVehicles.WheeledVehiclePawn|GetVehicleMovementComponent _aswheeled_vehicle_pawn) true)
      (Class|ChaosVehicleMovementComponent|SetSteeringInput (Variables|/Script/ChaosVehicles.WheeledVehiclePawn|GetVehicleMovementComponent _aswheeled_vehicle_pawn) 1.0)
      (bind _assports_car_pawn (Utilities|Casting|CastToSportsCar_Pawn (Game|Player|GetPlayerPawn 0)))
      (Audio|Components|Audio|Stop (Variables|/Game/VehicleTemplate/Blueprints/SportsCar/SportsCar_Pawn.SportsCar_Pawn_C|GetSFX_CarEngine _assports_car_pawn)))
    (:then_1
      (bind _outactors (Actor|GetAllActorsOfClass "/Script/LevelSequence.LevelSequenceActor"))
      (for _array_element _outactors
        (if (>= (Utilities|Array|FindItem (Variables|/Script/Engine.Actor|GetTags _array_element) (select Win (Utilities|Name|MakeLiteralName "Win") (Utilities|Name|MakeLiteralName "Lose"))) 0)
          (Sequencer|Player|Play (Variables|/Script/LevelSequence.LevelSequenceActor|GetSequencePlayer _array_element) :!class /Script/MovieScene.MovieSceneSequencePlayer))))))

(event Custom|Game%20Start
  (bind _returnvalue (Utilities|Time|SetTimerbyEvent (delegate Custom|Lose_OutOfTimeCounter) (Variables|Default|GetStartTimerDuration)))
  (Variables|Default|SetTimeRemainingTimer _returnvalue))

(event Custom|ReadyState
  (bind _returnvalue (Game|GetPlayerController 0))
  (Development|PrintString "Ready...Get....Set.....GO!!!")
  (Variables|/Script/Engine.PlayerController|SetbShowMouseCursor _returnvalue false)
  (Input|SetInputModeGameOnly _returnvalue false))

(event Custom|Lose_OutOfTimeCounter
  (bind _returnvalue (UserInterface|CreateWidget "/Game/MyGame/UI/WBP_LoseScreen.WBP_LoseScreen_C"))
  (UserInterface|Viewport|AddtoViewport _returnvalue 0)
  (Variables|/Script/Engine.PlayerController|SetbShowMouseCursor (Game|GetPlayerController 0) true)
  (CallFunction|GameFinish false))

(event Custom|Win_CrossedTheFinishLine
  (Utilities|Time|ClearandInvalidateTimerbyHandle (Variables|Default|GetTimeRemainingTimer))
  (bind _returnvalue (UserInterface|CreateWidget "/Game/MyGame/UI/WBP_WinScreen.WBP_WinScreen_C"))
  (UserInterface|Viewport|AddtoViewport _returnvalue 0)
  (Variables|/Script/Engine.PlayerController|SetbShowMouseCursor (Game|GetPlayerController 0) true)
  (CallFunction|GameFinish true))

(event Custom|CrossedCheckpoint
  (params (TimeToAdd :type Integer))
  (CallFunction|AddTimetoTimer TimeToAdd))

(event EventBeginPlay
  (Utilities|FlowControl|Sequence
    (:then_0
      (bind _outactors (Actor|GetAllActorsOfClass "/Game/MyGame/Chackpoints/BP_Checkpoint.BP_Checkpoint_C"))
      (for _array_element _outactors
        (if (Variables|/Game/MyGame/Chackpoints/BP_Checkpoint.BP_Checkpoint_C|GetisFinishLine _array_element)
          (EventDispatchers|BindEventtoOnCheckpointCrossed _array_element (EventDispatchers|CreateEvent :!event Custom|Win_CrossedTheFinishLine))
          (else
            (EventDispatchers|BindEventtoOnCheckpointCrossedwithTime _array_element (EventDispatchers|CreateEvent :!event Custom|CrossedCheckpoint))))))
    (:then_1
      (CallFunction|ReadyState))))

(fn ConstructionScript)

(fn AddTimetoTimer
  (params (TimeToAdd :type Integer))
  (bind _returnvalue (Utilities|Time|SetTimerbyEvent (EventDispatchers|CreateEvent :!event Custom|Lose_OutOfTimeCounter) (+ (Utilities|Time|GetTimerRemainingTimebyHandle (Variables|Default|GetTimeRemainingTimer)) TimeToAdd)))
  (Variables|Default|SetTimeRemainingTimer _returnvalue)
  (bind _asvehicle_player_controller (Utilities|Casting|CastToVehiclePlayerController (Game|GetPlayerController 0)))
  (Default|PlayAnimwhenTimeAdded (Variables|/Game/VehicleTemplate/Blueprints/VehiclePlayerController.VehiclePlayerController_C|GetVehicleHud _asvehicle_player_controller)))